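; BP_CharacterDiablo is a player character Blueprint with axis-driven movement and a montage-based attack.
; Each Tick, an input-check macro passes only non-zero axis input, which becomes the controller's rotation, and the character moves along the controller's forward vector.
; The Attack action plays the Warrior montage's Attack section only from the default state, switching to an attacking state until the AttackEnd event resets it.
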(event Custom|AttackEnd
  ;[1 1 1] 공격 종료
  (Variables|Default|SetStateBP "NewEnumerator0"))

(event EventTick
  (params (DeltaSeconds :type Float%20%28single-precision%29))
  ;[1 1 1] 캐릭터 이동
  (|입력확인)
  (Pawn|SetControlRotation (Game|GetPlayerController 0) (Math|Rotator|MakeRotfromX (Math|Vector|MakeVector (Input|AxisValues|GetUpDown) (Input|AxisValues|GetLeftRight) 0.0)))
  (Pawn|Input|AddMovementInput (Transformation|GetActorForwardVector (Game|GetPlayerController 0)) 1.0 false))

(event Input|ActionEvents|InputActionAttack
  (params (Key :type Key%20Structure))
  ;[1 1 1] 공격 전환
  (:Pressed
    (if (Utilities|Enum|Equal(Enum) (Variables|Default|GetStateBP) "NewEnumerator0")
      (Variables|Default|SetStateBP "NewEnumerator1")
      (Animation|PlayAnimMontage "/Game/Blueprint/Warrior_Montage.Warrior_Montage" 1.0 "Attack"))))

(fn ConstructionScript)