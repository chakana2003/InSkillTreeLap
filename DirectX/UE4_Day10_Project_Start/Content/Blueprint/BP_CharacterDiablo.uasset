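; Player character for a Diablo-style game, with movement, a basic attack and a cooldown-gated skill.
; Each Tick with nonzero axis input points the control rotation along the input and moves along the controller's forward vector.
; A state enum gates attack and skill, which play sections of one montage until their end events reset it.
; BP_CharacterController, cached on BeginPlay, checks and starts the skill cooldown.
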(event Custom|AttackEnd
  ;[1 1 1] 공격 종료
  (Variables|Default|SetStateBP "NewEnumerator0"))

(event Custom|DoAttack
  ;[1 1 1] 공격 전환
  (if (Utilities|Enum|Equal(Enum) (Variables|Default|GetStateBP) "NewEnumerator0")
    (Variables|Default|SetStateBP "NewEnumerator1")
    (Animation|PlayAnimMontage "/Game/Blueprint/Warrior_Montage.Warrior_Montage" 1.0 "Attack")))

(event Custom|DoSkill
  ;[1 1 1] 스킬 공격
  (bind _can_skill (Default|CanUseSkill (Variables|Default|GetRefController)))
  (if (and (Utilities|Enum|Equal(Enum) (Variables|Default|GetStateBP) "NewEnumerator0") _can_skill)
    (Variables|Default|SetStateBP "NewEnumerator1")
    (Animation|PlayAnimMontage "/Game/Blueprint/Warrior_Montage.Warrior_Montage" 1.0 "Skill")
    (Default|StartSkillCooldown (Variables|Default|GetRefController))))

(event Custom|SkillEnd
  ;[1 1 1] 스킬 종료
  (Variables|Default|SetStateBP "NewEnumerator0"))

(event EventBeginPlay
  ;[1 1 1] 컨트롤러 값 저장.
  (bind _asbp_character_controller (Utilities|Casting|CastToBP_CharacterController (Game|GetPlayerController 0)))
  (Variables|Default|SetRefController _asbp_character_controller))

(event EventTick
  (params (DeltaSeconds :type Float%20%28single-precision%29))
  ;[1 1 1] 캐릭터 이동
  (|입력확인)
  (Pawn|SetControlRotation (Game|GetPlayerController 0) (Math|Rotator|MakeRotfromX (Math|Vector|MakeVector (Input|AxisValues|GetUpDown) (Input|AxisValues|GetLeftRight) 0.0)))
  (Pawn|Input|AddMovementInput (Transformation|GetActorForwardVector (Game|GetPlayerController 0)) 1.0 false))

(event Input|ActionEvents|InputActionAttack
  (params (Key :type Key%20Structure))
  ;[1 1 1] 공격 전환
  (:Pressed
    (if (Utilities|Enum|Equal(Enum) (Variables|Default|GetStateBP) "NewEnumerator0")
      (Variables|Default|SetStateBP "NewEnumerator1")
      (Animation|PlayAnimMontage "/Game/Blueprint/Warrior_Montage.Warrior_Montage" 1.0 "Attack"))))

(fn ConstructionScript)