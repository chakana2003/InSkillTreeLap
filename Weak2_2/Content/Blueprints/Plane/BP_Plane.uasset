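; Player-controlled plane pawn that flies constantly forward and fires rockets.
; Axis inputs pitch and roll the actor and adjust a clamped CurrentSpeed, while the fire action spawns BP_Rocket at the Arrow component.
; Tick feeds CurrentSpeed into FloatingPawnMovement's MaxSpeed and the spin rate of two propeller meshes.
; Forward motion uses AddMovementInput rather than actor offsets so collision applies.
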(event Custom|RotatePropeller
  (params (프로펠러 :type Static%20Mesh%20Component%20Object%20Reference))
  (Transformation|AddLocalRotation 프로펠러 (Math|Rotator|MakeRotator (* (Utilities|Time|GetWorldDeltaSeconds) (Variables|Default|GetPropellerSpeed)) 0.0 0.0) false false))

(event EventBeginPlay)

(event Collision|EventActorBeginOverlap
  (params (OtherActor :type Actor%20Object%20Reference)))

(event EventTick
  (params (DeltaSeconds :type Float%20%28single-precision%29))
  (Utilities|FlowControl|Sequence
    (:then_0
      ;[1 1 1] 프로펠러 회전
      (Utilities|FlowControl|Sequence ; 프로펠러 회전
        (:then_0
          (CallFunction|RotatePropeller (Variables|Default|GetStaticMesh2)))
        (:then_1
          (CallFunction|RotatePropeller (Variables|Default|GetStaticMesh1)))
        (:then_2
          (Variables|Default|SetPropellerSpeed (* (Variables|Default|GetCurrentSpeed) 3e+01)))))
    (:then_1
      (Pawn|Input|AddMovementInput (Transformation|GetActorForwardVector) 1.0 false) ; AddActorOffset 을 쓸 경우 물리엔진이나 콜리전이 적용받지 않는다.\n그래서 FloationgPawnMovement 같은 컴포넌트를 추가해서\nAddMovementInput을 사용해 이동해야 한다.
      (Variables|/Script/Engine.FloatingPawnMovement|SetMaxSpeed (Variables|Default|GetFloatingPawnMovement) (Variables|Default|GetCurrentSpeed)))))

(event Input|ActionEvents|InputActionFireRocket
  (params (Key :type Key%20Structure))
  (:Pressed
    (Game|SpawnActorfromClass "/Game/Blueprints/Plane/BP_Rocket.BP_Rocket_C" (Transformation|GetWorldTransform (Variables|Default|GetArrow)) "Undefined" 0 0)))

(event Input|AxisEvents|InputAxisTurnUp
  (params (AxisValue :type Float%20%28single-precision%29))
  ;[1 1 1] 회전
  (Transformation|AddActorLocalRotation (Math|Rotator|MakeRotator 0.0 AxisValue 0.0) false false))

(event Input|AxisEvents|InputAxisTurnRight
  (params (AxisValue :type Float%20%28single-precision%29))
  ;[1 1 1] 회전
  (Transformation|AddActorLocalRotation (Math|Rotator|MakeRotator AxisValue 0.0 0.0) false false))

(event Input|AxisEvents|InputAxisAccellate
  (params (AxisValue :type Float%20%28single-precision%29))
  ;[1 1 1] 가속&감속
  (Variables|Default|SetCurrentSpeed (Math|Float|Clamp(Float) (+ (* AxisValue 1e+02) (Variables|Default|GetCurrentSpeed)) 2e+02 5e+03)))

(fn ConstructionScript)