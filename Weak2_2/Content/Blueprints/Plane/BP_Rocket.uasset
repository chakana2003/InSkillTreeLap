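; BP_Rocket is a rocket projectile actor that explodes on contact and has a limited lifetime.
; On BeginPlay it attaches a fire emitter to its Arrow component and starts a timer that calls DestroyRocket to remove it silently after a few seconds.
; A Capsule overlap spawns an explosion with random rotation and scale, then destroys the actor.
; The graphs apply no damage and set no movement.
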(event OnComponentBeginOverlap(Capsule)
  (params (OverlappedComponent :type Primitive%20Component%20Object%20Reference) (OtherActor :type Actor%20Object%20Reference) (OtherComp :type Primitive%20Component%20Object%20Reference) (OtherBodyIndex :type Integer) (bFromSweep :type Boolean) (SweepResult :type Hit%20Result%20Structure%20%28by%20ref%29))
  (bind _returnvalue (Math|Random|RandomFloatinRange 0.0 3.6e+02))
  (Effects|SpawnEmitteratLocation "/Game/StarterContent/Particles/P_Explosion.P_Explosion" (Transformation|GetActorLocation) (Math|Rotator|MakeRotator _returnvalue _returnvalue _returnvalue) (Math|Conversions|ToVector(Float) (Math|Random|RandomFloatinRange 1e+01 15.0)))
  (Actor|DestroyActor))

(event EventBeginPlay
  (Utilities|Time|SetTimerbyFunctionName self "DestroyRocket" 5.0)
  (Effects|SpawnEmitterAttached "/Game/StarterContent/Particles/P_Fire2.P_Fire2" (Variables|Default|GetArrow) "None"))

(event Collision|EventActorBeginOverlap
  (params (OtherActor :type Actor%20Object%20Reference)))

(event EventTick
  (params (DeltaSeconds :type Float%20%28single-precision%29)))

(fn ConstructionScript)

(fn DestroyRocket
  (Actor|DestroyActor))