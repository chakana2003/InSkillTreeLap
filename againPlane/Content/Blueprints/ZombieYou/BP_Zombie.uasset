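; Player-controlled zombie character with movement, camera zoom, jump, two attacks, two actions and a hold-to-ragdoll toggle.
; Input events set state flags that are not cleared here; Tick disables input during attacks or actions and stores the cardinal movement Direction.
; Action2 is a roll that Tick drives per frame, offsetting the actor forward while spinning and raising the mesh.
; Ragdoll reparents the spring arm to the simulated mesh, then moves the actor there on release.
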(event EventBeginPlay)

(event Collision|EventActorBeginOverlap
  (params (OtherActor :type Actor%20Object%20Reference)))

(event EventTick
  (params (DeltaSeconds :type Float%20%28single-precision%29))
  (bind _returnvalue (Transformation|GetActorRotation))
  (bind _returnvalue_2 (Transformation|GetActorRotation))
  (bind _returnvalue_3 (Input|AxisValues|GetMoveFoward))
  (bind _returnvalue_4 (Input|AxisValues|GetMoveRight))
  (bind _returnvalue_5 (Math|Vector|MakeVector _returnvalue_3 _returnvalue_4 0.0))
  (bind _returnvalue_6 (Math|Vector|GetForwardVector _returnvalue_2))
  (bind _returnvalue_7 (Math|Vector|GetRightVector _returnvalue_2))
  (bind _returnvalue_8 (Math|Vector|NegateVector _returnvalue_6))
  (bind _returnvalue_9 (Math|Vector|NegateVector _returnvalue_7))
  (Utilities|FlowControl|Sequence
    (:then_0
      ;[1 1 1] 현재 입력받은 방향 Vector 저장
      (if (Math|Vector|Equal(Vector) _returnvalue_5 "1.000000, 0, 0" 0.1)
        (Variables|Default|SetDirection _returnvalue_6)
        (elif (Math|Vector|Equal(Vector) _returnvalue_5 "-1.000000, 0, 0" 0.1)
          (Variables|Default|SetDirection (Math|Vector|MakeVector (.x _returnvalue_8) (.y _returnvalue_8) 0.0))
          (elif (Math|Vector|Equal(Vector) _returnvalue_5 "0.000000,1.000000, 0" 0.1)
            (Variables|Default|SetDirection _returnvalue_7)
            (elif (Math|Vector|Equal(Vector) _returnvalue_5 "0,-1.000000, 0" 0.1)
              (Variables|Default|SetDirection (Math|Vector|MakeVector (.x _returnvalue_9) (.y _returnvalue_9) 0.0)))))))
    (:then_1
      ;[1 1 1] 공격 & 액션 중 Input Disable
      (if (Math|Boolean|ORBoolean (Variables|Action|GetIsMainAttack) (Variables|Action|GetIsSubAttack) (Variables|Action|GetIsAction1) (Variables|Action|GetIsAction2))
        (Input|DisableInput 0)
        (else
          (Input|EnableInput 0))))
    (:then_2
      ;[1 1 1] 구르기
      (if (Variables|Action|GetIsAction2)
        (Utilities|FlowControl|Sequence
          (:then_0
            (Transformation|AddActorLocalOffset (* (Math|Vector|GetForwardVector (Math|Rotator|MakeRotator (.roll _returnvalue) (.pitch _returnvalue) 0.0)) 20) false false))
          (:then_1
            (Transformation|SetRelativeRotation (Variables|Character|GetMesh) (Math|Rotator|Lerp(Rotator) "0,-90.000000,90.000000" "0.000000,-90.000000,550.000000" (Variables|Rolling|GetRollingAlpha)) false false)
            (Transformation|SetRelativeLocation (Variables|Character|GetMesh) "0,0.000000,-40.000000" false false))
          (:then_2
            (Variables|Rolling|SetRollingAlpha (Math|Float|Clamp(Float) (+ (Variables|Rolling|GetRollingAlpha) 0.012)))))
        (else
          (Transformation|SetRelativeRotation (Variables|Character|GetMesh) "0,-90.000000, 0" false false)
          (Transformation|SetRelativeLocation (Variables|Character|GetMesh) "0.000000,0.000000,-90.000000" false false))))))

(event Input|ActionEvents|InputActionAction1
  (params (Key :type Key%20Structure))
  (:Pressed
    (Variables|Action|SetIsAction1 true)))

(event Input|ActionEvents|InputActionAction2
  (params (Key :type Key%20Structure))
  (:Pressed
    (Variables|Action|SetIsAction2 true)
    (Variables|Rolling|SetRollingAlpha 0.0)))

(event Input|ActionEvents|InputActionMainAttack
  (params (Key :type Key%20Structure))
  (:Pressed
    (Variables|Action|SetIsMainAttack true)))

(event Input|ActionEvents|InputActionSubAttack
  (params (Key :type Key%20Structure))
  (:Pressed
    (Variables|Action|SetIsSubAttack true)))

(event Input|ActionEvents|InputActionJump
  (params (Key :type Key%20Structure))
  (:Pressed
    (if (not (AI|Components|NavMovement|IsFalling (Variables|Character|GetCharacterMovement)))
      (Character|Jump)
      (Variables|Action|SetisJump true))))

(event Input|ActionEvents|InputActionDoll
  (params (Key :type Key%20Structure))
  (bind _mesh (Variables|Character|GetMesh))
  (bind _returnvalue (Transformation|GetWorldLocation _mesh))
  (:Pressed
    (Physics|SetSimulatePhysics (Variables|Character|GetMesh) true)
    (Collision|SetCollisionEnabled (Variables|Character|GetMesh) "QueryAndPhysics")
    (Transformation|AttachComponentToComponent (Variables|Default|GetSpringArm) (Variables|Character|GetMesh) "None" "KeepRelative" "KeepRelative" "KeepRelative" true))
  (:Released
    (Physics|SetSimulatePhysics _mesh false)
    (Transformation|SetActorLocation (Math|Vector|MakeVector (.x _returnvalue) (.y _returnvalue) (+ (.z _returnvalue) 5e+01)) false false)
    (Transformation|AttachComponentToComponent _mesh (Variables|Collision|GetCapsuleComponent) "None" "KeepRelative" "KeepRelative" "KeepRelative" true)
    (Transformation|SetRelativeLocation _mesh "0, 0,0.000000" false false)
    (Transformation|AttachComponentToComponent (Variables|Default|GetSpringArm) (Variables|Collision|GetCapsuleComponent) "None" "KeepRelative" "KeepRelative" "KeepRelative" true)))

(event Input|AxisEvents|InputAxisMoveFoward
  (params (AxisValue :type Float%20%28single-precision%29))
  (Pawn|Input|AddMovementInput (Transformation|GetActorForwardVector) (Math|Float|Clamp(Float) AxisValue -0.5) false))

(event Input|AxisEvents|InputAxisTurnRate
  (params (AxisValue :type Float%20%28single-precision%29))
  (Pawn|Input|AddControllerYawInput AxisValue))

(event Input|AxisEvents|InputAxisZoomRate
  (params (AxisValue :type Float%20%28single-precision%29))
  (Variables|/Script/Engine.SpringArmComponent|SetTargetArmLength (Variables|Default|GetSpringArm) (Math|Float|Clamp(Float) (+ AxisValue (Variables|/Script/Engine.SpringArmComponent|GetTargetArmLength (Variables|Default|GetSpringArm))) 1e+02 1e+03)))

(event Input|AxisEvents|InputAxisLookUpRate
  (params (AxisValue :type Float%20%28single-precision%29))
  (Pawn|Input|AddControllerPitchInput AxisValue))

(event Input|AxisEvents|InputAxisMoveRight
  (params (AxisValue :type Float%20%28single-precision%29))
  (Pawn|Input|AddMovementInput (Transformation|GetActorRightVector) AxisValue false))

(fn ConstructionScript)