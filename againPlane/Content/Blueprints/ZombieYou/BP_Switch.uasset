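; BP_Switch is a pressure-style switch actor whose mesh moves while something is inside its trigger box.
; Box begin overlap plays a timeline whose vector track sets the StaticMesh relative location, and end overlap reverses it.
; Any overlapping actor triggers it without filtering, and each overlap prints the actor's name with an enter or leave debug message.
; Disconnected nodes retain earlier instant-move and manual Lerp attempts that never run.
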(event OnComponentBeginOverlap(Box)
  (params (OverlappedComponent :type Primitive%20Component%20Object%20Reference) (OtherActor :type Actor%20Object%20Reference) (OtherComp :type Primitive%20Component%20Object%20Reference) (OtherBodyIndex :type Integer) (bFromSweep :type Boolean) (SweepResult :type Hit%20Result%20Structure%20%28by%20ref%29))
  (Development|PrintString (Utilities|GetDisplayName OtherActor))
  (Development|PrintString "들어옴")
  (bind _새_트랙_3 (Timeline|타임라인_0 Play)
    (:Update
      (Transformation|SetRelativeLocation (Variables|Default|GetStaticMesh) _새_트랙_3 false false))))

(event OnComponentEndOverlap(Box)
  (params (OverlappedComponent :type Primitive%20Component%20Object%20Reference) (OtherActor :type Actor%20Object%20Reference) (OtherComp :type Primitive%20Component%20Object%20Reference) (OtherBodyIndex :type Integer))
  (Development|PrintString (Utilities|GetDisplayName OtherActor))
  (Development|PrintString "나감")
  (bind _새_트랙_3 (Timeline|타임라인_0 Reverse)
    (:Update
      (Transformation|SetRelativeLocation (Variables|Default|GetStaticMesh) _새_트랙_3 false false))))

(event EventBeginPlay)

(event Collision|EventActorBeginOverlap
  (params (OtherActor :type Actor%20Object%20Reference)))

(event EventTick
  (params (DeltaSeconds :type Float%20%28single-precision%29)))

(fn ConstructionScript)