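; BP_Plane is a player-controlled plane pawn that flies continuously forward and can fire rockets.
; Tick feeds full movement input along the forward vector, while the Accelete axis adjusts FloatingPawnMovement's MaxSpeed, scaled by delta time and clamped, to act as a throttle.
; Pitch and roll axes apply local rotation directly, without delta-time scaling, steering the flight direction.
; FireRocket spawns a BP_Rocket at the Arrow component's world transform.
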(event EventBeginPlay)

(event Collision|EventActorBeginOverlap
  (params (OtherActor :type Actor%20Object%20Reference)))

(event EventTick
  (params (DeltaSeconds :type Float%20%28single-precision%29))
  (Pawn|Input|AddMovementInput (Transformation|GetActorForwardVector) 1.0 false))

(event Input|ActionEvents|InputActionFireRocket
  (params (Key :type Key%20Structure)))

(event Input|ActionEvents|InputActionFireRocket
  (params (Key :type Key%20Structure))
  (:Pressed
    (Game|SpawnActorfromClass "/Game/Blueprints/Plane/BP_Rocket.BP_Rocket_C" (Transformation|GetWorldTransform (Variables|Default|GetArrow)) "Undefined" 0 0)))

(event Input|AxisEvents|InputAxisTurnPitch
  (params (AxisValue :type Float%20%28single-precision%29))
  (Transformation|AddActorLocalRotation (Math|Rotator|MakeRotator 0.0 AxisValue 0.0) false false))

(event Input|AxisEvents|InputAxisAccelete
  (params (AxisValue :type Float%20%28single-precision%29))
  (Variables|/Script/Engine.FloatingPawnMovement|SetMaxSpeed (Variables|Default|GetFloatingPawnMovement) (Math|Float|Clamp(Float) (+ (* (* AxisValue 1e+04) (Utilities|Time|GetWorldDeltaSeconds)) (Class|MovementComponent|GetMaxSpeed (Variables|Default|GetFloatingPawnMovement))) 5e+02 5e+03)))

(event Input|AxisEvents|InputAxisTurnRoll
  (params (AxisValue :type Float%20%28single-precision%29))
  (Transformation|AddActorLocalRotation (Math|Rotator|MakeRotator AxisValue 0.0 0.0) false false))

(fn ConstructionScript)