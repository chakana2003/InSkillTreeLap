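; P-38 plane actor that moves with player axis input and spins its two propellers.
; MoveForward and MoveRight add raw axis values as local X and Y offsets, without delta-time scaling.
; Each Tick derives MinSpeed from MaxSpeed, then calls the 회전 (rotate) function on both propellers.
; That function rolls a propeller by delta time times a random speed within that range, so spin varies every frame.
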(event EventTick
  (params (DeltaSeconds :type Float%20%28single-precision%29))
  (Utilities|FlowControl|Sequence
    (:then_0
      (Variables|프로펠러|SetMinSpeed (- (Variables|프로펠러|GetMaxSpeed) 5e+02)))
    (:then_1
      ;[1 1 1] 프로펠러 회전
      (Utilities|FlowControl|Sequence
        (:then_0
          (CallFunction|회전 (Variables|Default|GetPropels1)))
        (:then_1
          (CallFunction|회전 (Variables|Default|GetPropels2)))))))

(event Input|AxisEvents|InputAxisMoveRight
  (params (AxisValue :type Float%20%28single-precision%29))
  (Transformation|AddActorLocalOffset (Math|Vector|MakeVector 0.0 AxisValue 0.0) false false))

(event Input|AxisEvents|InputAxisMoveForward
  (params (AxisValue :type Float%20%28single-precision%29))
  (Transformation|AddActorLocalOffset (Math|Vector|MakeVector AxisValue 0.0 0.0) false false))

(fn ConstructionScript)

(fn 회전
  (params (프로펠러 :type Static%20Mesh%20Component%20Object%20Reference))
  (Transformation|AddRelativeRotation 프로펠러 (Math|Rotator|MakeRotator (* (Utilities|Time|GetWorldDeltaSeconds) (Math|Random|RandomFloatinRange (Variables|프로펠러|GetMinSpeed) (Variables|프로펠러|GetMaxSpeed))) 0.0 0.0) false false))